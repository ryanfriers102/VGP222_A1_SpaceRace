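; BP_JediFighter is a player-flown starfighter driven by physics on its ShipMesh.
; Thrust input eases speed toward a target along the mesh's right vector, with Boost raising that target well beyond MaxThrust through unclamped Lerp.
; Tick overwrites linear velocity with forward velocity plus a second term, gravity-based below GravityThreshold and interpolated from forward velocity otherwise.
; MoveUp, MoveSide and Roll steer by applying heavily scaled torque about mesh axes.
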(event `InputAction|Boost`
  (params (Key :type "Key Structure"))
  (:`Pressed`
    (set `self.Boost` true))
  (:`Released`
    (set `self.Boost` false)))

(event `InputAxis|Thrust`
  (params (AxisValue :type "Float (single-precision)"))
  (`|ExecutionSequence`
    (:`then_0`
      (if (`self.Boost`)
        (if (not (`KismetMathLibrary.NearlyEqual_FloatFloat` AxisValue 0.0 0.1))
          (set `self.Thrust` (`KismetMathLibrary.FInterpTo` (`self.Thrust`) (`KismetMathLibrary.Lerp` 0.0 (`self.MaxThrust`) (/ (+ AxisValue 1.0) 0.2)) (`GameplayStatics.GetWorldDeltaSeconds`) 0.5)))
        (elif (not (`KismetMathLibrary.NearlyEqual_FloatFloat` AxisValue 0.0 0.1))
          (set `self.Thrust` (`KismetMathLibrary.FInterpTo` (`self.Thrust`) (`KismetMathLibrary.Lerp` 0.0 (`self.MaxThrust`) (/ (+ AxisValue 1.0) 2.0)) (`GameplayStatics.GetWorldDeltaSeconds`) 0.5)))))
    (:`then_1`
      (set `self.ForwardVelocity` (* (`SceneComponent.GetRightVector` (`self.Ship_Mesh`)) (`self.Thrust`))))))

(event `self.ReceiveTick`
  (params (DeltaSeconds :type "Float (single-precision)"))
  (`|ExecutionSequence`
    (:`then_0`
      (if (< (`KismetMathLibrary.VSize` (`self.ForwardVelocity`)) (`self.GravityThreshold`))
        (set `self.UpwardsVelocity` (* (`KismetMathLibrary.Lerp` 0.0 -980.0 (- (`KismetMathLibrary.VSize` (`self.ForwardVelocity`)) (`self.GravityThreshold`))) (`KismetMathLibrary.LessLess_VectorRotator` (`SceneComponent.GetUpVector` (`self.Ship_Mesh`)) (`SceneComponent.K2_GetComponentRotation` (`self.Ship_Mesh`)))))
        (else
          (set `self.UpwardsVelocity` (`KismetMathLibrary.VInterpTo` (`self.ForwardVelocity`) (0.0 0.0 0.0) (`GameplayStatics.GetWorldDeltaSeconds`) 20.0)))))
    (:`then_1`
      (`PrimitiveComponent.SetPhysicsLinearVelocity` (`self.Ship_Mesh`) (+ (`self.ForwardVelocity`) (`self.UpwardsVelocity`)) false "None"))))

(event `InputAxis|MoveUp`
  (params (AxisValue :type "Float (single-precision)"))
  (`PrimitiveComponent.AddTorqueInDegrees` (`self.Ship_Mesh`) (* (* AxisValue (`self.ForwardTorquePower`)) (`SceneComponent.GetForwardVector` (`self.Ship_Mesh`)) 3000000000.0) "None" false))

(event `InputAxis|MoveSide`
  (params (AxisValue :type "Float (single-precision)"))
  (`PrimitiveComponent.AddTorqueInDegrees` (`self.Ship_Mesh`) (* (* AxisValue (`self.ForwardTorquePower`)) (`SceneComponent.GetUpVector` (`self.Ship_Mesh`)) 3000000000.0) "None" false))

(event `InputAxis|Roll`
  (params (AxisValue :type "Float (single-precision)"))
  (`PrimitiveComponent.AddTorqueInDegrees` (`self.Ship_Mesh`) (* (* AxisValue (`self.SideTorquePower`)) (`SceneComponent.GetRightVector` (`self.Ship_Mesh`)) -3000000000.0) "None" false))

(fn `UserConstructionScript`)