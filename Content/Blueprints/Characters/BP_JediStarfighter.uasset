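; Jedi starfighter ship Blueprint that adds thruster visuals on top of its parent class's behavior.
; Each tick runs the parent logic, then slides ThrusterRoot along its local Y axis in proportion to Thrust over MaxNormalThrust, clamped to a fixed range.
; The Boost input switches the ThrusterColor parameter on both thruster effects to blue while held and to purple on release.
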(event `self.ReceiveTick`
  (params (DeltaSeconds :type "Float (single-precision)"))
  (bind _thrusterroot (`self.ThrusterRoot`))
  (bind (_relativelocation_x _relativelocation_y _relativelocation_z) (`KismetMathLibrary.BreakVector` (`SceneComponent.RelativeLocation` _thrusterroot)))
  (`parent.ReceiveTick` DeltaSeconds)
  (`SceneComponent.K2_SetRelativeLocation` _thrusterroot (`KismetMathLibrary.MakeVector` _relativelocation_x (`KismetMathLibrary.FClamp` (* (+ (* (/ (`self.Thrust`) (`self.MaxNormalThrust`)) 10000.0) 15000.0) -1.0) -25000.0 -15000.0) _relativelocation_z) false false))

(event `InputAction|Boost` :overrideparent false
  (params (Key :type "Key Structure"))
  (bind _ns_thrustereffect1 (`self.NS_ThrusterEffect1`))
  (:`Pressed`
    (`FXSystemComponent.SetColorParameter` _ns_thrustereffect1 "ThrusterColor" (struct :`G` 0.462526 :`B` 1.0 :`A` 1.0))
    (`FXSystemComponent.SetColorParameter` (`self.NS_ThrusterEffect`) "ThrusterColor" (struct :`G` 0.462526 :`B` 1.0 :`A` 1.0)))
  (:`Released`
    (`FXSystemComponent.SetColorParameter` _ns_thrustereffect1 "ThrusterColor" (struct :`R` 0.486588 :`B` 1.0 :`A` 1.0))
    (`FXSystemComponent.SetColorParameter` (`self.NS_ThrusterEffect`) "ThrusterColor" (struct :`R` 0.486588 :`B` 1.0 :`A` 1.0))))

(fn `UserConstructionScript`
  (`parent.UserConstructionScript`))