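; Game mode that tracks hoop completions and ends the level once enough hoops are cleared.
; On BeginPlay it creates the WB_HUD widget and adds it to the viewport.
; HoopCompleted increments a counter and calls GameOver when it reaches MaxHoops.
; GameOver starts a camera fade and immediately opens the MainMenu level, without waiting for the fade to finish.
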(event `self.ReceiveBeginPlay`
  (bind _returnvalue (`|CreateWidget` "/Game/Blueprints/Widgets/WB_HUD.WB_HUD_C"))
  (`UserWidget.AddToViewport` _returnvalue 0))

(fn `GameOver`
  (`KismetSystemLibrary.PrintString` "Game Over!")
  (`PlayerCameraManager.StartCameraFade` :`self` (`GameplayStatics.GetPlayerCameraManager` 0) :`ToAlpha` 1.0 :`Duration` 2.0)
  (`GameplayStatics.OpenLevel` "MainMenu"))

(fn `HoopCompleted`
  (set `self.HoopsCompleted` (+ (`self.HoopsCompleted`) 1))
  (`KismetSystemLibrary.PrintString` "Hoop Completed")
  (if (>= (`self.HoopsCompleted`) (`self.MaxHoops`))
    (`self.GameOver`)))

(fn `UserConstructionScript`)